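; Turtle NPC Blueprint that spawns with sound and particle effects and moves under AI control.
; On BeginPlay it plays spawn effects, attaches movement sound and emitter to its Body, then spawns a default controller and runs the Turtle_BT behavior tree.
; A DespawnTurtle event plays despawn sound and particles at its location before destroying the actor.
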(event `self.ReceiveBeginPlay`
  (`self.Spawn Sounds and effects`)
  ;[1 1 1] Giving Turtle AI Controller
  (`self.SpawnDefaultController`)
  (`AIController.RunBehaviorTree` (`AIBlueprintHelperLibrary.GetAIController` self) "/Game/Blueprints/Turtle_NPC/Turtle_BT.Turtle_BT"))

(event `Spawn Sounds and effects`
  (bind _returnvalue (`self.K2_GetActorLocation`))
  (bind _body (`self.Body`))
  ;[1 1 1] Giving Turtle sounds and effects
  (`GameplayStatics.PlaySoundAtLocation` "/Game/Sounds/Turtle_spawn.Turtle_spawn" _returnvalue (struct) 1.0 1.0 0.0 null null null)
  (`GameplayStatics.SpawnSoundAttached` "/Game/Sounds/Turtle_move.Turtle_move" _body "None" (0.0 0.0 0.0) (struct) "KeepRelativeOffset" true 1.0 1.0 0.0 null null)
  (`GameplayStatics.SpawnEmitterAtLocation` "/Game/Effects/Turtle_Spawn_PS.Turtle_Spawn_PS" _returnvalue)
  (`GameplayStatics.SpawnEmitterAttached` "/Game/Effects/Turtle_Move_PS.Turtle_Move_PS" _body))

(event `Despawn Turtle`
  (bind _returnvalue (`self.K2_GetActorLocation`))
  ;[1 1 1] Despawning Turtle with sounds and effects
  (`GameplayStatics.PlaySoundAtLocation` "/Game/Sounds/Turtle_despawn.Turtle_despawn" _returnvalue (struct) 1.0 1.0 0.0 null null null)
  (`GameplayStatics.SpawnEmitterAtLocation` "/Game/Effects/Turtle_Despawn_PS.Turtle_Despawn_PS" _returnvalue)
  (`self.K2_DestroyActor`))

(fn `UserConstructionScript`)