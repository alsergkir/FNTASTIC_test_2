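; Player Blueprint that handles movement, look and interaction input.
; Movement axes add input along the actor's forward and right vectors, and look axes drive controller pitch and yaw.
; Pressing Use scans overlapping actors and sends InteractMessage to the first one implementing Interact_BPI, so interactable objects define their own response through the interface.
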(event `InputAxis|MoveForward`
  (params (AxisValue :type "Float (single-precision)"))
  ;[1 1 1] Player movement
  (`self.AddMovementInput` (`self.GetActorForwardVector`) AxisValue))

(event `InputAxis|MoveRight`
  (params (AxisValue :type "Float (single-precision)"))
  ;[1 1 1] Player movement
  (`self.AddMovementInput` (`self.GetActorRightVector`) AxisValue))

(event `InputAxis|LookVertical`
  (params (AxisValue :type "Float (single-precision)"))
  ;[1 1 1] Player movement
  (`self.AddControllerPitchInput` AxisValue))

(event `InputAxis|LookHorizontal`
  (params (AxisValue :type "Float (single-precision)"))
  ;[1 1 1] Player movement
  (`self.AddControllerYawInput` AxisValue))

(event `InputAction|Use`
  (params (Key :type "Key Structure"))
  ;[1 1 1] Player interaction ('E' and 'LMB')
  (:`Pressed`
    (for _array_element (`self.GetOverlappingActors` null)
      (if (`KismetSystemLibrary.DoesImplementInterface` _array_element "/Game/Blueprints/Interact_BPI.Interact_BPI_C")
        (message `/Game/Blueprints/Interact_BPI.Interact` _array_element)
        (break)))))

(fn `UserConstructionScript`)